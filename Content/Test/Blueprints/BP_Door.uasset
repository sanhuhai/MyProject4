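; BP_Door is a test door actor that reacts to BP_Player entering and leaving a box trigger.
; Overlap begin calls OpenDoor, which only sets IsOpen, with no timeline playback wired.
; Overlap end calls CloseDoor, which reverses TL_OpenDoor to lerp the door's yaw when IsOpen is true.
; IsOpen is cleared only in the already-closed branch, so it stays true after first opening, and debug strings are printed.
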(event `OpenDoor`
  (if (`self.bIsOpen`)
    (`KismetSystemLibrary.PrintString` "alerady open!!!")
    (else
      (set `self.bIsOpen` true))))

(event `CloseDoor`
  (if (`self.bIsOpen`)
    (bind (_direction _alpha) (`Timeline|TL_OpenDoor` :!via `Reverse`)
      (:`Update`
        (`SceneComponent.K2_SetRelativeRotation` (`self.Door`) (`KismetMathLibrary.MakeRotator` 0.0 0.0 (`KismetMathLibrary.Lerp` 0.0 90.0 _alpha)) false false))
      (:`Finished`
        (`KismetSystemLibrary.PrintString` "Carry out!!!")))
    (else
      (set `self.bIsOpen` false)
      (`KismetSystemLibrary.PrintString` "alerady close!!!"))))

(event `self.Box.OnComponentBeginOverlap`
  (params (OverlappedComponent :type "PrimitiveComponent Object Reference") (OtherActor :type "Actor Object Reference") (OtherComp :type "PrimitiveComponent Object Reference") (OtherBodyIndex :type Integer) (bFromSweep :type Boolean) (SweepResult :type "HitResult Structure (by ref)"))
  (cast `/Game/Test/Blueprints/BP_Player` OtherActor)
  (`self.OpenDoor`))

(event `self.Box.OnComponentEndOverlap`
  (params (OverlappedComponent :type "PrimitiveComponent Object Reference") (OtherActor :type "Actor Object Reference") (OtherComp :type "PrimitiveComponent Object Reference") (OtherBodyIndex :type Integer))
  (cast `/Game/Test/Blueprints/BP_Player` OtherActor)
  (`self.CloseDoor`))

(fn `UserConstructionScript`)