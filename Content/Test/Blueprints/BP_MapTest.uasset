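; BP_MapTest is a test Blueprint that exercises string-to-integer map operations and prints the results.
; On BeginPlay it binds PrintMap to the VirtualBox OnTriggerVirtual event, and PrintMap calls MapOperator.
; MapOperator prints each key with its value, removes the "one" entry, then prints the remaining values and a completion message.
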(event `self.ReceiveBeginPlay`
  (add `/Game/Test/Blueprints/BP_VirtualBox.OnTriggerVirtual` (`self.VirtualBox`) (delegate `PrintMap`)))

(event `PrintMap`
  (`self.MapOperator`))

(event `MapOperator`
  (bind _mystringintegermap (`self.MyStringIntegerMap`))
  (bind _keys (`BlueprintMapLibrary.Map_Keys` (`self.MyStringIntegerMap`)))
  (for _array_element _keys
    (`KismetSystemLibrary.PrintString` (`KismetStringLibrary.Concat_StrStr` _array_element (`KismetStringLibrary.Conv_IntToString` (`BlueprintMapLibrary.Map_Find` (`self.MyStringIntegerMap`) _array_element)))))
  (`BlueprintMapLibrary.Map_Remove` _mystringintegermap "one")
  (bind _values (`BlueprintMapLibrary.Map_Values` _mystringintegermap))
  (for _array_element_2 _values
    (`KismetSystemLibrary.PrintString` (`KismetStringLibrary.Conv_IntToString` _array_element_2)))
  (`KismetSystemLibrary.PrintString` "complent"))

(fn `UserConstructionScript`)